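; Balrog actor Blueprint that dresses itself with a light and fire particle effects on BeginPlay.
; It spawns a light actor at the "Light Source" mesh socket and attaches it to itself.
; A loop spawns fire actors at numbered "Fire Particles" sockets until one is missing.
; The counter increments before each attach, so the attach socket name uses the next index.
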(event EventBeginPlay
  (bind _self self)
  (bind _returnvalue (Game|SpawnActorfromClass "/Game/MyContent/Blueprints/Balrog/BalrogLightBP.BalrogLightBP_C" (Transformation|GetSocketTransform (Variables|Character|GetMesh) "Light Source" "RTS_World") "AlwaysSpawn" _self 0))
  (Class|Actor|AttachRootComponenttoActor _returnvalue _self "Light Source" "KeepWorldPosition" true)
  (while (> (Variables|Default|GetCurrent%20Fire%20Socket) 0)
    (if (Transformation|DoesSocketExist (Variables|Character|GetMesh) (Utilities|String|StringToName (Utilities|String|Append (Utilities|String|MakeLiteralString "Fire Particles ") (Utilities|String|ToString(Integer) (Variables|Default|GetCurrent%20Fire%20Socket)))))
      (bind _returnvalue_2 (Game|SpawnActorfromClass "/Game/MyContent/Blueprints/Balrog/BalrogFirePaticlesBP.BalrogFirePaticlesBP_C" (Transformation|GetSocketTransform (Variables|Character|GetMesh) (Utilities|String|StringToName (Utilities|String|Append (Utilities|String|MakeLiteralString "Fire Particles ") (Utilities|String|ToString(Integer) (Variables|Default|GetCurrent%20Fire%20Socket)))) "RTS_World") "AlwaysSpawn" self 0))
      (Math|Integer|IncrementInt (Variables|Default|GetCurrent%20Fire%20Socket)
        (:%20%20
          (Class|Actor|AttachRootComponenttoActor _returnvalue_2 self (Utilities|String|StringToName (Utilities|String|Append (Utilities|String|MakeLiteralString "Fire Particles ") (Utilities|String|ToString(Integer) (Variables|Default|GetCurrent%20Fire%20Socket)))) "KeepWorldPosition" true)))
      (else
        (Variables|Default|SetCurrent%20Fire%20Socket -99)))))

(fn ConstructionScript)